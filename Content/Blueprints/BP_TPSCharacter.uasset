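; Third-person shooter character Blueprint that handles the overhead net role display and the sniper scope overlay.
; On BeginPlay it passes itself to the overhead widget to show the player's net role.
; ShowSniperScope lazily creates the scope widget on first call, then plays its zoom animation forward or in reverse with matching zoom-in or zoom-out sounds.
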(event `self.ReceiveBeginPlay`
  (bind _aswbp_overhead_widget (cast `/Game/Blueprints/HUD/WBP_OverheadWidget` (`WidgetComponent.GetUserWidgetObject` (`self.overheadWidget`))))
  (`OverheadWidget.ShowPlayerNetRole` _aswbp_overhead_widget self))

(event `self.ShowSniperScope`
  (params (_bShow :type Boolean))
  (bind _sniperscope (`self.SniperScope`))
  (bind _sniperscope_2 (`self.SniperScope`))
  (`/Engine/EditorBlueprintResources/StandardMacros.IsValid` (`self.SniperScope`)
    (:`Is Valid`
      _)
    (:`Is Not Valid`
      (bind _returnvalue (`|CreateWidget` "/Game/Blueprints/HUD/WBP_SniperScope.WBP_SniperScope_C"))
      (bind _output_get (set `self.SniperScope` _returnvalue))
      (`UserWidget.AddToViewport` _output_get 0)))
  (if _bShow
    (`/Engine/EditorBlueprintResources/StandardMacros.IsValid` _sniperscope_2
      (:`Is Valid`
        (`UserWidget.PlayAnimation` _sniperscope_2 (`/Game/Blueprints/HUD/WBP_SniperScope.ScopeZommIn` _sniperscope_2) 0.0 1 "Forward" 1.0 false)
        (`GameplayStatics.PlaySound2D` "/Game/AssetPack/MilitaryWeapSilver/Sound/SniperRifle/Cues/SniperRifle_ZoomIn_Cue.SniperRifle_ZoomIn_Cue" 1.0 1.0 0.0 null null)))
    (else
      (`/Engine/EditorBlueprintResources/StandardMacros.IsValid` _sniperscope
        (:`Is Valid`
          (`UserWidget.PlayAnimation` _sniperscope (`/Game/Blueprints/HUD/WBP_SniperScope.ScopeZommIn` _sniperscope) 0.0 1 "Reverse" 1.0 false)
          (`GameplayStatics.PlaySound2D` "/Game/AssetPack/MilitaryWeapSilver/Sound/SniperRifle/Cues/SniperRifle_ZoomOut_Cue.SniperRifle_ZoomOut_Cue" 1.0 1.0 0.0 null null))))))

(fn `UserConstructionScript`)